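; Networked player character with movement, a two-hit sword combo, equipment visuals and ragdoll death.
; On possession it initializes BPPlayerStats from PlayerState base plus adjust stats, spawns a socketed sword, restores equipped meshes and caches GameMode skill data.
; Attacks go client-to-server then multicast, with a timed input window for the combo and PoseState freezing acceleration while attacking or dead.
; Equipment meshes replicate through OnRep handlers, and damage feeds the stats component.
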(event `self.ReceiveBeginPlay`
  (set `self.Orient Rotation To Movement` (`CharacterMovementComponent.bOrientRotationToMovement` (`self.CharacterMovement`)))
  ; 죽었을 때 이벤트 바인딩
  (add `/Game/Blueprints/InGame/Components/BP_CharacterStats.OnDead` (`self.BP_PlayerStats`) (`|CreateDelegate` :!event `Dead`)))

(event `self.ReceivePossessed`
  (params (NewController :type "Controller Object Reference"))
  (`|ExecutionSequence`
    (:`then_0`
      (bind _asbp_player_state (cast `/Game/Blueprints/InGame/Character/BP_PlayerState` (`Controller.PlayerState` NewController)))
      (bind _output_get (set `self.Ref_PlayerState` _asbp_player_state))
      (bind _returnvalue (`DataLibrary.AddCharacterStats` (`/Game/Blueprints/InGame/Character/BP_PlayerState.BaseStats` _output_get) (`/Game/Blueprints/InGame/Character/BP_PlayerState.AdjustStats` _output_get)))
      ; 기본 체력 설정
      (`/Game/Blueprints/InGame/Components/BP_CharacterStats.InitStats` (`self.BP_PlayerStats`) _returnvalue _returnvalue))
    (:`then_1`
      ; 검 장착
      (`/Engine/EditorBlueprintResources/StandardMacros.IsValid` (`self.Ref_Sword`)
        (:`Is Not Valid`
          (bind _returnvalue_2 (`|SpawnActorFromClass` "/Game/Blueprints/InGame/Item/BP_Sword.BP_Sword_C" (`KismetMathLibrary.MakeTransform` (0.0 0.0 0.0)) "Undefined" "MultiplyWithRoot" self self))
          (bind _output_get_2 (set `self.Ref_Sword` _returnvalue_2))
          (`self.K2_AttachToComponent` _output_get_2 (`self.Mesh`) "SwordSocket" "KeepRelative" "KeepRelative" "KeepWorld" true))))
    (:`then_2`
      ; 아이템 슬롯만큼 메시 공간 할당
      (`KismetArrayLibrary.Array_Resize` (`self.EquippedMeshs`) (enumcount `/Game/Blueprints/InGame/Datas/Enum/E_ItemSlot`))
      ; 착용한 아이템 메쉬 업데이트
      (`/Game/Blueprints/InGame/Character/BP_PlayerState.AttachCurrentAllItemMesh` (`self.Ref_PlayerState`))
      ; 죽었을 때 서버 이벤트
      (add `/Game/Blueprints/InGame/Components/BP_CharacterStats.Server_OnDead` (`self.BP_PlayerStats`) (`|CreateDelegate` (`self.Ref_PlayerState`) :!event `OnDead`))
      ; 서버에서 받아온 스킬 데이터 저장
      (bind _asbp_gamemode (cast `/Game/Blueprints/InGame/Core/BP_Gamemode` (`GameplayStatics.GetGameMode`)))
      (set `self.SkillList` (`/Game/Blueprints/InGame/Core/BP_Gamemode.SkillAssetDatas` _asbp_gamemode)))))

(event `CallAttackInput`
  ; 공격
  (if (`|EnumInequality` (`self.PoseState`) "Dead")
    (`self.C2S_Attack`)))

(event `C2S_Attack`
  ; 공격
  (switch `EState` (`self.PoseState`)
    (:`Normal`
      (`self.S2M_Attack` false))
    (:`Attack`
      (`self.S2M_Attack` true))))

(event `S2M_Attack`
  (params (IsAttacking :type Boolean))
  ; 공격
  (if IsAttacking
    (set `self.CachedAttackedTime` (`GameplayStatics.GetTimeSeconds`))
    (else
      (`self.PlayAnimMontage` "/Game/Animation/AM_SwordAttack.AM_SwordAttack" 1.0 "Attack1")
      (`self.SetMovementFromState` "Attack")
      (set `self.CachedAttackedTime` (`GameplayStatics.GetTimeSeconds`)))))

(event `C2S_CheckCombo`
  ; 콤보 체크
  ;; 공격했던 시간이 짧다면 다음 콤보공격
  (if (`|EnumEquality` (`self.PoseState`) "Attack")
    (`self.S2M_CheckCombo` (<= (- (`GameplayStatics.GetTimeSeconds`) (`self.CachedAttackedTime`)) 0.5))
    (else
      (`self.S2M_CheckCombo` false))))

(event `S2M_CheckCombo`
  (params (IsComboSuccess :type Boolean))
  ; 콤보 체크
  (if IsComboSuccess
    (`|PlayMontage` (`self.Mesh`) "/Game/Animation/AM_SwordAttack.AM_SwordAttack" 1.0 0.0 "Attack2"
      (:`OnCompleted`
        _)
      (:`OnInterrupted`
        _)))
  (`self.SetMovementFromState` "Normal")
  (set `self.CachedAttackedTime` 0.0))

(event `self.ReceiveAnyDamage`
  (params (Damage :type "Float (single-precision)") (DamageType :type "DamageType Object Reference") (InstigatedBy :type "Controller Object Reference") (DamageCauser :type "Actor Object Reference"))
  (`/Game/Blueprints/InGame/Components/BP_CharacterStats.TakeAnyDamage` (`self.BP_PlayerStats`) (`KismetMathLibrary.FTrunc` Damage)))

(fn `AttachItemMesh`
  (params (InItemSlot :type "/Game/Blueprints/InGame/Datas/Enum/E_ItemSlot Enum" :default "NewEnumerator0") (InSkeletalMesh :type "SkeletalMesh Object Reference"))
  (bind _equippedmeshs (`self.EquippedMeshs`))
  ; 무기 종류라면 칼 소켓 비우기
  (if (`|EnumEquality` InItemSlot "NewEnumerator6")
    (`self.DetachSwordMesh`))
  (`KismetArrayLibrary.Array_Set` _equippedmeshs (`KismetMathLibrary.Conv_ByteToInt` InItemSlot) InSkeletalMesh)
  (set `self.EquippedMeshs` _equippedmeshs))

(fn `AttachSwordMesh`
  (params (InItemSlot :type "/Game/Blueprints/InGame/Datas/Enum/E_ItemSlot Enum" :default "NewEnumerator0") (InSwordMesh :type "StaticMesh Object Reference"))
  (`self.DetachItemMesh` InItemSlot)
  (bind _output_get (set `self.EquippedSwordMesh` (`local.InSwordMesh`)))
  (`/Game/Blueprints/InGame/Item/BP_Sword.SetSwordMesh` (`self.Ref_Sword`) _output_get))

(fn `Dead`
  ; 충돌처리 해제
  (`PrimitiveComponent.SetCollisionEnabled` (`self.Mesh`) "PhysicsOnly")
  (`PrimitiveComponent.SetCollisionEnabled` (`self.CapsuleComponent`) "NoCollision")
  ; 랙돌효과
  (`PrimitiveComponent.SetSimulatePhysics` (`self.Mesh`) true))

(fn `DetachItemMesh`
  (params (InItemSlot :type "/Game/Blueprints/InGame/Datas/Enum/E_ItemSlot Enum" :default "NewEnumerator0"))
  (`KismetArrayLibrary.Array_Set` (`self.EquippedMeshs`) (`KismetMathLibrary.Conv_ByteToInt` InItemSlot))
  (`self.SetItemSlotMeshes`))

(fn `DetachSwordMesh`
  (bind _output_get (set `self.EquippedSwordMesh` null))
  (`/Game/Blueprints/InGame/Item/BP_Sword.SetSwordMesh` (`self.Ref_Sword`) _output_get))

(fn `LookUp`
  (params (Value :type "Float (double-precision)"))
  (`self.AddControllerPitchInput` Value))

(fn `Move`
  (params (IsForward :type Boolean) (AxisValue :type "Float (double-precision)"))
  (bind (_returnvalue_roll _returnvalue_pitch _returnvalue_yaw) (`KismetMathLibrary.BreakRotator` (`self.GetControlRotation`)))
  (bind _returnvalue (`KismetMathLibrary.MakeRotator` 0.0 0.0 _returnvalue_yaw))
  (if IsForward
    (`self.AddMovementInput` (`KismetMathLibrary.GetForwardVector` _returnvalue) AxisValue)
    (else
      (`self.AddMovementInput` (`KismetMathLibrary.GetRightVector` _returnvalue) AxisValue))))

(fn `OnRep_EquippedMeshs`
  (`self.SetItemSlotMeshes`))

(fn `OnRep_EquippedSwordMesh`
  (bind _ref_sword (`self.Ref_Sword`))
  (`/Engine/EditorBlueprintResources/StandardMacros.IsValid` _ref_sword
    (:`Is Valid`
      (`/Game/Blueprints/InGame/Item/BP_Sword.SetSwordMesh` _ref_sword (`self.EquippedSwordMesh`)))))

(fn `ProcessJump`
  (`self.Jump`))

(fn `SetItemSlotMeshes`
  (bind _enumvalue (foreach `/Game/Blueprints/InGame/Datas/Enum/E_ItemSlot` false)
    (:`LoopBody`
      (`SkeletalMeshComponent.SetSkeletalMeshAsset` (select `/Game/Blueprints/InGame/Datas/Enum/E_ItemSlot` _enumvalue :`NewEnumerator0` (`self.HeadSlotMesh`) :`NewEnumerator3` (`self.ChestSlotMesh`) :`NewEnumerator6` (`self.WeaponSlotMesh`)) (`|GetArrayItem` (`self.EquippedMeshs`) (`KismetMathLibrary.Conv_ByteToInt` _enumvalue))))))

(fn `SetMovementFromState`
  (params (InPoseState :type "EState Enum" :default "Normal"))
  (bind _output_get (set `self.PoseState` InPoseState))
  (switch `EState` _output_get
    (:`Normal`
      (set `CharacterMovementComponent.MaxAcceleration` 2048.0 (`self.CharacterMovement`)))
    (:`Attack`
      (set `CharacterMovementComponent.MaxAcceleration` 0.0 (`self.CharacterMovement`) :!label _label))
    (:`Dead`
      (goto _label))))

(fn `Turn`
  (params (Value :type "Float (double-precision)"))
  (`self.AddControllerYawInput` Value))

(fn `UserConstructionScript`)