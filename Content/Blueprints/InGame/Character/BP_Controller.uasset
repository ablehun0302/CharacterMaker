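; Player controller that turns input into character movement, camera look, attacks, skill use and HUD skill/inventory toggles.
; Item equip, skill slot changes, skill use and restart go through C2S events to BP_PlayerState or BP_Gamemode, with restart allowed only when dead.
; Pawn changes rebind the HUD and hide its restart button, while unpossessing destroys the player's sword.
; Player and PlayerState references are lazily cached through getters.
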(event `self.ReceiveBeginPlay`
  (bind _asbp_hud (cast `/Game/Blueprints/InGame/Core/BP_HUD` (`self.GetHUD`)))
  (set `self.Ref_HUD` _asbp_hud)
  (`WidgetBlueprintLibrary.SetInputMode_GameOnly` self)
  (set `self.bShowMouseCursor` false)
  (add `self.OnPossessedPawnChanged` (delegate `CustomEvent`)))

(event `CustomEvent` :!signature `self.OnPossessedPawnChanged`
  (params (OldPawn :type "Pawn Object Reference") (NewPawn :type "Pawn Object Reference"))
  (`/Game/Blueprints/InGame/Core/BP_HUD.BindPlayerEvent` (`self.Ref_HUD`))
  (`/Game/Blueprints/InGame/Core/BP_HUD.HideRestartButton` (`self.Ref_HUD`)))

(event `self.ReceiveUnPossess`
  (params (UnpossessedPawn :type "Pawn Object Reference"))
  (bind _asbp_player (cast `/Game/Blueprints/InGame/Character/BP_Player` UnpossessedPawn))
  (bind _ref_sword (`/Game/Blueprints/InGame/Character/BP_Player.Ref_Sword` _asbp_player)
    (:`then`
      (`self.K2_DestroyActor` _ref_sword))
    (:`else`)))

(event `InputAxis|MoveForward`
  (params (AxisValue :type "Float (single-precision)"))
  (bind _outplayer (`self.GetBP_Player`))
  ; 이동
  (`/Engine/EditorBlueprintResources/StandardMacros.IsValid` _outplayer
    (:`Is Valid`
      (`/Game/Blueprints/InGame/Character/BP_Player.Move` _outplayer true AxisValue))))

(event `InputAxis|Turn`
  (params (AxisValue :type "Float (single-precision)"))
  ; 회전
  (if (not (`self.bShowMouseCursor`))
    (`self.AddYawInput` AxisValue)))

(event `InputAxis|MoveRight`
  (params (AxisValue :type "Float (single-precision)"))
  (bind _outplayer (`self.GetBP_Player`))
  ; 이동
  (`/Engine/EditorBlueprintResources/StandardMacros.IsValid` _outplayer
    (:`Is Valid`
      (`/Game/Blueprints/InGame/Character/BP_Player.Move` _outplayer false AxisValue))))

(event `InputAxis|LookUp`
  (params (AxisValue :type "Float (single-precision)"))
  ; 회전
  (if (not (`self.bShowMouseCursor`))
    (`self.AddPitchInput` AxisValue)))

(event `InputAction|SkillTree`
  (params (Key :type "Key Structure"))
  ; UI
  (:`Pressed`
    (if (not (`/Game/Blueprints/InGame/Character/BP_PlayerState.bIsDead` (`self.GetBP_PlayerState`)))
      (`/Game/Blueprints/InGame/Core/BP_HUD.ToggleSkillUI` (`self.Ref_HUD`)))))

(event `InputAction|Jump`
  (params (Key :type "Key Structure"))
  ; 점프
  (:`Pressed`
    (`Character.Jump` (`self.GetBP_Player`))))

(event `InputAction|Inventory`
  (params (Key :type "Key Structure"))
  ; UI
  (:`Pressed`
    (if (not (`/Game/Blueprints/InGame/Character/BP_PlayerState.bIsDead` (`self.GetBP_PlayerState`)))
      (`/Game/Blueprints/InGame/Core/BP_HUD.ToggleItemUI` (`self.Ref_HUD`)))))

(event `CallItemSelected`
  (params (InIndex :type Integer))
  ; 아이템 선택 시
  (`self.C2S_ItemSelected` InIndex))

(event `C2S_ItemSelected`
  (params (InIndex :type Integer))
  (`/Engine/EditorBlueprintResources/StandardMacros.IsValid` (`self.K2_GetPawn`)
    (:`Is Valid`
      (`/Game/Blueprints/InGame/Character/BP_PlayerState.EquipItem` (`self.GetBP_PlayerState`) InIndex))))

(event `CallDetatchItem`
  (params (InItemSlot :type "/Game/Blueprints/InGame/Datas/Enum/E_ItemSlot Enum" :default "NewEnumerator0"))
  ; 아이템 해제시
  (`self.C2S_DetatchItem` InItemSlot))

(event `C2S_DetatchItem`
  (params (InItemSlot :type "/Game/Blueprints/InGame/Datas/Enum/E_ItemSlot Enum" :default "NewEnumerator0"))
  (`/Engine/EditorBlueprintResources/StandardMacros.IsValid` (`self.K2_GetPawn`)
    (:`Is Valid`
      (`/Game/Blueprints/InGame/Character/BP_PlayerState.UnequipItem` (`self.GetBP_PlayerState`) InItemSlot))))

(event `InputAction|MainSkill`
  (params (Key :type "Key Structure"))
  ; 스킬
  (:`Pressed`
    (`self.C2S_Skill` "NewEnumerator1")))

(event `C2S_Skill`
  (params (InSkillSlot :type "/Game/Blueprints/InGame/Datas/Enum/E_SkillSlot Enum" :default "NewEnumerator0"))
  (bind _outplayerstate (`self.GetBP_PlayerState`))
  (`/Engine/EditorBlueprintResources/StandardMacros.IsValid` _outplayerstate
    (:`Is Valid`
      (`/Game/Blueprints/InGame/Character/BP_PlayerState.UseSkill` _outplayerstate InSkillSlot))))

(event `InputAction|SubSkill`
  (params (Key :type "Key Structure"))
  ; 스킬
  (:`Pressed`
    (`self.C2S_Skill` "NewEnumerator0")))

(event `CallOnAttatchSkill`
  (params (InIndex :type Integer) (InSkillSlot :type "/Game/Blueprints/InGame/Datas/Enum/E_SkillSlot Enum" :default "NewEnumerator0"))
  ; 선택한 스킬 장착 시
  (`self.C2S_AttatchSkill` InIndex InSkillSlot))

(event `C2S_AttatchSkill`
  (params (InIndex :type Integer) (InSkillSlot :type "/Game/Blueprints/InGame/Datas/Enum/E_SkillSlot Enum" :default "NewEnumerator0"))
  ; 선택한 스킬 장착 시
  (bind _asbp_gamemode (cast `/Game/Blueprints/InGame/Core/BP_Gamemode` (`GameplayStatics.GetGameMode`)))
  (`/Game/Blueprints/InGame/Core/BP_Gamemode.GetSkillData` _asbp_gamemode self InIndex InSkillSlot))

(event `CallOnDetatchSkill`
  (params (InSkillSlot :type "/Game/Blueprints/InGame/Datas/Enum/E_SkillSlot Enum" :default "NewEnumerator0"))
  ; 스킬 장착 해제 시
  (`self.C2S_DetatchSkill` InSkillSlot))

(event `C2S_DetatchSkill`
  (params (InSkillSlot :type "/Game/Blueprints/InGame/Datas/Enum/E_SkillSlot Enum" :default "NewEnumerator0"))
  ; 스킬 장착 해제 시
  (`/Engine/EditorBlueprintResources/StandardMacros.IsValid` (`self.K2_GetPawn`)
    (:`Is Valid`
      (`/Game/Blueprints/InGame/Character/BP_PlayerState.DetatchSkill` (`self.GetBP_PlayerState`) InSkillSlot))))

(event `InputAction|Attack`
  (params (Key :type "Key Structure"))
  (bind _ref_player (`self.Ref_Player`))
  (:`Pressed`
    (`/Engine/EditorBlueprintResources/StandardMacros.IsValid` _ref_player
      (:`Is Valid`
        (`/Game/Blueprints/InGame/Character/BP_Player.CallAttackInput` _ref_player)))))

(event `C2S_Restart`
  ; 리스폰
  (if (`/Game/Blueprints/InGame/Character/BP_PlayerState.bIsDead` (`self.GetBP_PlayerState`))
    (bind _asbp_gamemode (cast `/Game/Blueprints/InGame/Core/BP_Gamemode` (`GameplayStatics.GetGameMode`)))
    (`/Game/Blueprints/InGame/Core/BP_Gamemode.RestartClient` _asbp_gamemode self)))

(event `CallOnRestart`
  ; 리스폰
  (if (`/Game/Blueprints/InGame/Character/BP_PlayerState.bIsDead` (`self.GetBP_PlayerState`))
    (`self.C2S_Restart`)))

(fn `GetBP_Player`
  (returns (OutPlayer :type "/Game/Blueprints/InGame/Character/BP_Player Object Reference"))
  (`/Engine/EditorBlueprintResources/StandardMacros.IsValid` (`self.Ref_Player`)
    (:`Is Valid`
      (return (`self.Ref_Player`)))
    (:`Is Not Valid`
      (bind _asbp_player (cast `/Game/Blueprints/InGame/Character/BP_Player` (`self.K2_GetPawn`))
        (:`then`
          (bind _output_get (set `self.Ref_Player` _asbp_player))
          (return _output_get))
        (:`CastFailed`
          (return null))))))

(fn `GetBP_PlayerState`
  (returns (OutPlayerState :type "/Game/Blueprints/InGame/Character/BP_PlayerState Object Reference"))
  (`/Engine/EditorBlueprintResources/StandardMacros.IsValid` (`self.Ref_PlayerState`)
    (:`Is Valid`
      (return (`self.Ref_PlayerState`)))
    (:`Is Not Valid`
      (bind _asbp_player_state (cast `/Game/Blueprints/InGame/Character/BP_PlayerState` (`self.PlayerState`)))
      (bind _output_get (set `self.Ref_PlayerState` _asbp_player_state))
      (return _output_get))))

(fn `UserConstructionScript`)