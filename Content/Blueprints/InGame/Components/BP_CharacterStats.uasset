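; Player character stats component that holds replicated current and max stats, applies damage and handles death.
; Max stat updates swap an old adjustment for a new one, and both these updates and damage clamp current stats to the maximum.
; Damage that empties Health triggers OnDead on the owning BP_PlayerState for server-side death.
; RepNotifies on both stat sets broadcast changes for UI and fire a death event at zero Health.
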(fn `GetOwnPlayer`
  (returns (OutBP_Player :type "/Game/Blueprints/InGame/Character/BP_Player Object Reference"))
  (`/Engine/EditorBlueprintResources/StandardMacros.IsValid` (`self.Ref_Player`)
    (:`Is Valid`
      (return (`self.Ref_Player`)))
    (:`Is Not Valid`
      (bind _asbp_player (cast `/Game/Blueprints/InGame/Character/BP_Player` (`self.GetOwner`)))
      (bind _output_get (set `self.Ref_Player` _asbp_player))
      (return _output_get))))

(fn `InitStats`
  (params (InCurrentStats :type "CharacterStats Structure") (InMaxStats :type "CharacterStats Structure"))
  (set `self.CurrentStats` InCurrentStats)
  (set `self.MaxStats` InMaxStats))

(fn `OnRep_CurrentStats`
  (`self.OnRepFunc_AllStats`))

(fn `OnRep_MaxStats`
  (`self.OnRepFunc_AllStats`))

(fn `OnRepFunc_AllStats`
  (`|ExecutionSequence`
    (:`then_0`
      ; UI 변경
      (`self.OnChangedStats` (`self.CurrentStats`) (`self.MaxStats`)))
    (:`then_1`
      ; 체력이 0 이하인지 확인
      (if (<= (`.Health` (break `CharacterStats` (`self.CurrentStats`))) 0)
        ; 리스폰 UI, 죽었을 때 클라 이벤트
        (`self.OnDead`)))))

(fn `TakeAnyDamage`
  (params (InDamage :type Integer))
  (bind _returnvalue (`DataLibrary.SetCharacterStatFromType` (`self.CurrentStats`) "Health" (* InDamage -1)))
  (bind _returnvalue_2 (`DataLibrary.ClampCharacterStats` _returnvalue (`self.MaxStats`)))
  (`|ExecutionSequence`
    (:`then_0`
      ; 현재 스탯 반영 전 체력이 0 이하인지 확인
      (if (<= (`DataLibrary.GetCharacterStatFromType` _returnvalue_2 "Health") 0)
        ; 서버측 죽음 처리
        (bind _asbp_player_state (cast `/Game/Blueprints/InGame/Character/BP_PlayerState` (`Pawn.PlayerState` (`self.GetOwnPlayer`))))
        (`/Game/Blueprints/InGame/Character/BP_PlayerState.OnDead` _asbp_player_state null)))
    (:`then_1`
      (set `self.CurrentStats` _returnvalue_2))))

(fn `UpdateMaxStats`
  (params (InPreAdjustStats :type "CharacterStats Structure") (InAdjustStats :type "CharacterStats Structure"))
  ; Max Stat 변경
  (bind _output_get (set `self.MaxStats` (`DataLibrary.AddCharacterStats` (`DataLibrary.SubtractCharacterStats` (`self.MaxStats`) (`local.InPreAdjustStats`)) (`local.InAdjustStats`))))
  (bind _returnvalue (`DataLibrary.ClampCharacterStats` (`self.CurrentStats`) _output_get))
  (set `self.CurrentStats` _returnvalue))