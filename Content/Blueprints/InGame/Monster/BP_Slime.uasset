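; BP_Slime is a slime monster character that takes damage and handles its death.
; A BPMonsterStats component is initialized from base stats on the server and receives incoming damage as whole numbers, with an event bound to its death notification.
; Dead switches the state enum, zeroes movement acceleration and writes the state to the BP_SlimeController blackboard for the AI.
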(event `self.ReceiveBeginPlay`
  (bind _basestats (`self.BaseStats`))
  (`|ExecutionSequence`
    (:`then_0`
      (`/Engine/EditorBlueprintResources/ActorMacros.Switch Has Authority`
        (:`Authority`
          (`/Game/Blueprints/InGame/Components/BP_CharacterStats.InitStats` (`self.BP_MonsterStats`) _basestats _basestats))))
    (:`then_1`
      (add `/Game/Blueprints/InGame/Components/BP_CharacterStats.OnDead` (`self.BP_MonsterStats`) (`|CreateDelegate` :!event `Dead`)))))

(event `self.ReceiveAnyDamage`
  (params (Damage :type "Float (single-precision)") (DamageType :type "DamageType Object Reference") (InstigatedBy :type "Controller Object Reference") (DamageCauser :type "Actor Object Reference"))
  (`/Game/Blueprints/InGame/Components/BP_CharacterStats.TakeAnyDamage` (`self.BP_MonsterStats`) (`KismetMathLibrary.FTrunc` Damage)))

(fn `Dead`
  (`self.SetCurrentState` "NewEnumerator3")
  (set `CharacterMovementComponent.MaxAcceleration` 0.0 (`self.CharacterMovement`))
  (bind _asbp_slime_controller (cast `/Game/Blueprints/InGame/Monster/BP_SlimeController` (`self.GetController`)))
  (`BlackboardComponent.SetValueAsEnum` (`AIBlueprintHelperLibrary.GetBlackboard` _asbp_slime_controller) "CurrentState" (`self.CurrentState`)))

(fn `SetCurrentState`
  (params (InCurrentState :type "/Game/Blueprints/InGame/Datas/Enum/E_MonsterState Enum" :default "NewEnumerator0"))
  (set `self.CurrentState` InCurrentState))

(fn `UserConstructionScript`)