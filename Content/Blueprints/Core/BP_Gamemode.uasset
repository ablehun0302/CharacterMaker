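; Game mode Blueprint that handles respawning players after death.
; RestartClient destroys the controlled BP_Player and its sword, then clears IsDead on the BP_PlayerState.
; It then spawns a new BP_Player at a found player start, owned by the controller, and possesses it.
; OnPlayerDead only fetches the dead player's pawn and takes no further action.
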(fn `OnPlayerDead`
  (params (InPlayerState :type "/Game/Blueprints/Core/BP_PlayerState Object Reference"))
  (locals (Ref_Pawn :type "Pawn Object Reference"))
  (set `local.Ref_Pawn` (`PlayerState.GetPawn` InPlayerState)))

(fn `RestartClient`
  (params (InPlayerController :type "PlayerController Object Reference"))
  (locals (Ref_DeadPawn :type "Pawn Object Reference"))
  ; 죽은 캐릭터 삭제
  (bind _asbp_player (cast `/Game/Blueprints/Character/BP_Player` (`Controller.K2_GetPawn` InPlayerController)))
  (`self.K2_DestroyActor` (`/Game/Blueprints/Character/BP_Player.Ref_Sword` _asbp_player))
  (`self.K2_DestroyActor` _asbp_player)
  ; 죽은 상태 초기화
  (bind _asbp_player_state (cast `/Game/Blueprints/Core/BP_PlayerState` (`Controller.PlayerState` (`local.InPlayerController`))))
  (set `/Game/Blueprints/Core/BP_PlayerState.bIsDead` false _asbp_player_state)
  ; 캐릭터 생성
  (bind _returnvalue (`|SpawnActorFromClass` "/Game/Blueprints/Character/BP_Player.BP_Player_C" (`self.GetTransform` (`self.K2_FindPlayerStart` (`local.InPlayerController`))) "Undefined" "MultiplyWithRoot" (`local.InPlayerController`) null))
  (`Controller.Possess` (`local.InPlayerController`) _returnvalue))

(fn `UserConstructionScript`)