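; BP_PlayerState holds a character's base and current stats, the stats of equipped items, and the list of available items.
; The construction script copies base stats to current, adds a zeroed stat entry per E_ItemSlot value, and loads every DT_Items row into ItemDatas.
; EquipItem writes the chosen item's stat adjustments at its slot's enum index, then rebuilds current stats from base plus all slots.
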(fn `EquipItem`
  (params (InIndex :type Integer))
  (bind (_output_itemid _output_itemname _output_slot _output_adjuststats) (break `/Game/Blueprints/Datas/Structure/ST_ItemInfo` (`|GetArrayItem` (`self.ItemDatas`) InIndex)))
  (`KismetArrayLibrary.Array_Set` (`self.EquippedItems`) (`KismetMathLibrary.Conv_ByteToInt` _output_slot) _output_adjuststats)
  ; 장착한 아이템 변경시 현재 스탯 업뎃
  (set `self.CurrentStats` (`self.BaseStats`))
  (for _array_element (`self.EquippedItems`)
    (set `self.CurrentStats` (`DataLibrary.AddCharacterStats` (`self.CurrentStats`) _array_element))))

(fn `UserConstructionScript`
  (`|ExecutionSequence`
    (:`then_0`
      ; 캐릭터 초기 스탯 초기화
      (set `self.CurrentStats` (`self.BaseStats`)))
    (:`then_1`
      ; 캐릭터 아이템 슬롯 초기화
      (foreach `/Game/Blueprints/Datas/Enum/E_ItemSlot` true
        (:`LoopBody`
          (`KismetArrayLibrary.Array_Add` (`self.EquippedItems`) (make `CharacterStats` 0.0)))))
    (:`then_2`
      ; 아이템 풀 초기화
      (bind _outrownames (`DataTableFunctionLibrary.GetDataTableRowNames` "/Game/Blueprints/Datas/DataTable/DT_Items.DT_Items"))
      (for _array_element _outrownames
        (bind _returnvalue (`|GetDataTableRow` "/Game/Blueprints/Datas/DataTable/DT_Items.DT_Items" _array_element)
          (:`then`
            (`KismetArrayLibrary.Array_Add` (`self.ItemDatas`) (make `/Game/Blueprints/Datas/Structure/ST_ItemInfo` _array_element (break `/Game/Blueprints/Datas/Structure/ST_ItemData` _returnvalue) (`.Slot_13_F1E0FF0D4685ADB0C5EC70993474033B` (break `/Game/Blueprints/Datas/Structure/ST_ItemData` _returnvalue)) (`.AdjustStats_9_288C978C4D8C40B55295F3B129592EB2` (break `/Game/Blueprints/Datas/Structure/ST_ItemData` _returnvalue)) (`.ItemMesh_20_56B5E5774D5F5B35A63BB1AF3D3F15E1` (break `/Game/Blueprints/Datas/Structure/ST_ItemData` _returnvalue)) (`.ItemImage_24_C9ADD5254F05D3E7C89801A47058A2AD` (break `/Game/Blueprints/Datas/Structure/ST_ItemData` _returnvalue))))))))))