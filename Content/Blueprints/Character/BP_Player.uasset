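; BP_Player is the player character Blueprint, providing camera-relative movement, look, jump and visible equipment for head, chest and weapon slots.
; Movement follows control yaw, with look and jump as thin wrappers.
; Attach and detach functions write to a RepNotify mesh array indexed by slot enum, then reapply every slot's skeletal mesh, as does the OnRep.
; Skill equip and unequip are empty stubs, and skill use holds only an unreachable missing-skill message.
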(event `self.ReceiveBeginPlay`
  (set `self.Orient Rotation To Movement` (`CharacterMovementComponent.bOrientRotationToMovement` (`self.CharacterMovement`)))
  (`KismetArrayLibrary.Array_Resize` (`self.EquippedMeshs`) (enumcount `/Game/Blueprints/Datas/Enum/E_ItemSlot`)))

(fn `AttatchItemMesh`
  (params (InItemSlot :type "/Game/Blueprints/Datas/Enum/E_ItemSlot Enum" :default "NewEnumerator0") (InSkeletalMesh :type "SkeletalMesh Object Reference"))
  (`KismetArrayLibrary.Array_Set` (`self.EquippedMeshs`) (`KismetMathLibrary.Conv_ByteToInt` InItemSlot) InSkeletalMesh)
  (`self.SetItemSlotMeshes`))

(fn `DetatchItemMesh`
  (params (InItemSlot :type "/Game/Blueprints/Datas/Enum/E_ItemSlot Enum" :default "NewEnumerator0"))
  (`KismetArrayLibrary.Array_Set` (`self.EquippedMeshs`) (`KismetMathLibrary.Conv_ByteToInt` InItemSlot))
  (`self.SetItemSlotMeshes`))

(fn `EquipSkill`
  (params (InSkillSlot :type "/Game/Blueprints/Datas/Enum/E_SkillSlot Enum" :default "NewEnumerator0") (InSkillBase :type "Object Object Reference")))

(fn `LookUp`
  (params (Value :type "Float (double-precision)"))
  (`self.AddControllerPitchInput` Value))

(fn `Move`
  (params (IsForward :type Boolean) (AxisValue :type "Float (double-precision)"))
  (bind (_returnvalue_roll _returnvalue_pitch _returnvalue_yaw) (`KismetMathLibrary.BreakRotator` (`self.GetControlRotation`)))
  (bind _returnvalue (`KismetMathLibrary.MakeRotator` 0.0 0.0 _returnvalue_yaw))
  (if IsForward
    (`self.AddMovementInput` (`KismetMathLibrary.GetForwardVector` _returnvalue) AxisValue)
    (else
      (`self.AddMovementInput` (`KismetMathLibrary.GetRightVector` _returnvalue) AxisValue))))

(fn `OnRep_EquippedMeshs`
  (`self.SetItemSlotMeshes`))

(fn `ProcessJump`
  (`self.Jump`))

(fn `SetItemSlotMeshes`
  (bind _enumvalue (foreach `/Game/Blueprints/Datas/Enum/E_ItemSlot` false)
    (:`LoopBody`
      (`SkeletalMeshComponent.SetSkeletalMeshAsset` (select `/Game/Blueprints/Datas/Enum/E_ItemSlot` _enumvalue :`NewEnumerator0` (`self.HeadSlotMesh`) :`NewEnumerator3` (`self.ChestSlotMesh`) :`NewEnumerator6` (`self.WeaponSlotMesh`)) (`|GetArrayItem` (`self.EquippedMeshs`) (`KismetMathLibrary.Conv_ByteToInt` _enumvalue))))))

(fn `Turn`
  (params (Value :type "Float (double-precision)"))
  (`self.AddControllerYawInput` Value))

(fn `UnequipSkill`
  (params (SkillSlot :type "/Game/Blueprints/Datas/Enum/E_SkillSlot Enum" :default "NewEnumerator0")))

(fn `UseActiveSkill`
  (params (SkillSlot :type "/Game/Blueprints/Datas/Enum/E_SkillSlot Enum" :default "NewEnumerator0"))
  (if (not true)
    (`KismetSystemLibrary.PrintText` (`|FormatText` "{0} 스킬이 없소" (`|GenericToText` (`local.SkillSlot`))) true true (struct :`R` 1.0 :`B` 0.01506 :`A` 1.0) 10.0)))

(fn `UserConstructionScript`)