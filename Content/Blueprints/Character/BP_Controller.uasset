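; Player controller that turns player input into character, camera and UI actions.
; BeginPlay caches BP_Player and BP_HUD, then input handlers forward movement, jump and main/sub skills to the player and skill-tree and inventory toggles to the HUD.
; Camera yaw and pitch input is ignored while the mouse cursor is shown.
; Item selection passes through a client-to-server (C2S) event that equips the chosen index on the pawn's BP_PlayerState.
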(event `self.ReceiveBeginPlay`
  (bind _asbp_player (cast `/Game/Blueprints/Character/BP_Player` (`self.K2_GetPawn`)))
  (set `self.PlayerRef` _asbp_player)
  (bind _asbp_hud (cast `/Game/Blueprints/Core/BP_HUD` (`self.GetHUD`)))
  (bind _output_get (set `self.As BP HUD` _asbp_hud))
  (`/Engine/EditorBlueprintResources/StandardMacros.IsValid` _output_get
    (:`Is Not Valid`
      (`KismetSystemLibrary.PrintString` "None BP HUD In BP Controller" true true (struct :`G` 0.66 :`B` 1.0 :`A` 1.0) 20.0))))

(event `InputAxis|MoveForward`
  (params (AxisValue :type "Float (single-precision)"))
  (bind _playerref (`self.PlayerRef`))
  ; 이동
  (`/Engine/EditorBlueprintResources/StandardMacros.IsValid` _playerref
    (:`Is Valid`
      (`/Game/Blueprints/Character/BP_Player.Move` _playerref true AxisValue))))

(event `InputAxis|Turn`
  (params (AxisValue :type "Float (single-precision)"))
  ; 회전
  (if (not (`self.bShowMouseCursor`))
    (`self.AddYawInput` AxisValue)))

(event `InputAxis|MoveRight`
  (params (AxisValue :type "Float (single-precision)"))
  (bind _playerref (`self.PlayerRef`))
  ; 이동
  (`/Engine/EditorBlueprintResources/StandardMacros.IsValid` _playerref
    (:`Is Valid`
      (`/Game/Blueprints/Character/BP_Player.Move` _playerref false AxisValue))))

(event `InputAxis|LookUp`
  (params (AxisValue :type "Float (single-precision)"))
  ; 회전
  (if (not (`self.bShowMouseCursor`))
    (`self.AddPitchInput` AxisValue)))

(event `InputAction|MainSkill`
  (params (Key :type "Key Structure"))
  ; 스킬
  (:`Pressed`
    (`/Game/Blueprints/Character/BP_Player.UseActiveSkill` (`self.PlayerRef`) "NewEnumerator1")))

(event `InputAction|Jump`
  (params (Key :type "Key Structure"))
  ; 점프
  (:`Pressed`
    (`Character.Jump` (`self.PlayerRef`))))

(event `InputAction|SubSkill`
  (params (Key :type "Key Structure"))
  ; 스킬
  (:`Pressed`
    (`/Game/Blueprints/Character/BP_Player.UseActiveSkill` (`self.PlayerRef`) "NewEnumerator0")))

(event `InputAction|SkillTree`
  (params (Key :type "Key Structure"))
  ; UI
  (:`Pressed`
    (`/Game/Blueprints/Core/BP_HUD.ToggleSkillUI` (`self.As BP HUD`))))

(event `InputAction|Inventory`
  (params (Key :type "Key Structure"))
  ; UI
  (:`Pressed`
    (`/Game/Blueprints/Core/BP_HUD.ToggleItemUI` (`self.As BP HUD`))))

(event `OnItemSelected`
  (params (InIndex :type Integer))
  ; 아이템 선택 시
  (`self.C2S_ItemSelected` InIndex))

(event `C2S_ItemSelected`
  (params (InIndex :type Integer))
  (bind _asbp_player_state (cast `/Game/Blueprints/Core/BP_PlayerState` (`Pawn.PlayerState` (`self.K2_GetPawn`))))
  (`/Engine/EditorBlueprintResources/StandardMacros.IsValid` _asbp_player_state
    (:`Is Valid`
      (`/Game/Blueprints/Core/BP_PlayerState.EquipItem` _asbp_player_state InIndex))))

(fn `UserConstructionScript`)