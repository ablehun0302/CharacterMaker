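; BP_SkillBase is a skill Blueprint, named as a base class, that holds a name, description, duration and ID.
; InitSkillBaseData fills these fields from its inputs, and ResetSkillBaseData restores them to "Null" strings and a zero duration.
; ProcessSkill only prints the skill name as text, using the skill's duration as the display time.
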(fn `InitSkillBaseData`
  (params (InName :type Text) (InDescription :type String) (InDuration :type "Float (double-precision)") (ID :type Name))
  (set `self.Name` InName)
  (set `self.Desctiption` InDescription)
  (set `self.Duration` InDuration)
  (set `self.ID` ID))

(fn `ProcessSkill`
  (`KismetSystemLibrary.PrintText` null (`self.Name`) true true (struct :`G` 0.66 :`B` 1.0 :`A` 1.0) (`self.Duration`)))

(fn `ResetSkillBaseData`
  (set `self.Name` "Null")
  (set `self.Desctiption` "Null")
  (set `self.Duration` 0.0)
  (set `self.ID` "Null"))