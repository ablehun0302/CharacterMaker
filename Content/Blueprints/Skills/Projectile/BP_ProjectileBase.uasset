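; Base projectile actor for skills, with a sphere collider, projectile movement and a Niagara particle.
; Its construction script configures collision size, movement, lifespan and bullet and hit effects from ProjectileSkillData.
; On a sphere hit, it spawns the pooled hit effect at the impact, deactivates the bullet particle and starts a short timer, apparently for delayed destruction.
; No damage logic is present here.
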(event `self.Sphere.OnComponentHit`
  (params (HitComponent :type "PrimitiveComponent Object Reference") (OtherActor :type "Actor Object Reference") (OtherComp :type "PrimitiveComponent Object Reference") (NormalImpulse :type "Vector Structure") (Hit :type "HitResult Structure (by ref)"))
  (`self.OnHit` Hit_Location))

(event `self.ReceiveDestroyed`)

(fn `OnDestroy`
  ; 투사체 자리에 부딪히는 파티클 생성
  (`self.K2_DestroyActor`))

(fn `OnHit`
  (params (Location :type "Vector Structure"))
  ; 투사체 자리에 부딪히는 파티클 생성
  (`NiagaraFunctionLibrary.SpawnSystemAtLocation` (`self.HitParticle`) Location (struct) (1.0 1.0 1.0) true true "AutoRelease")
  (`KismetSystemLibrary.K2_SetTimerDelegate` (`|CreateDelegate` :!event `OnDestroy`) 2.0)
  (`ActorComponent.Deactivate` (`self.Particle`)))

(fn `UserConstructionScript`
  (bind (_projectileskilldata_baseskilldata _projectileskilldata_bulletradius _projectileskilldata_speed _projectileskilldata_lifespan _projectileskilldata_gravityscale _projectileskilldata_bulletparticle _projectileskilldata_hitparticle) (break `ProjectileSkillData` (`self.ProjectileSkillData`)))
  (`SphereComponent.SetSphereRadius` (`self.Sphere`) _projectileskilldata_bulletradius true)
  (set `ProjectileMovementComponent.InitialSpeed` _projectileskilldata_speed (`self.ProjectileMovement`))
  (`self.SetLifeSpan` _projectileskilldata_lifespan)
  (set `ProjectileMovementComponent.ProjectileGravityScale` _projectileskilldata_gravityscale (`self.ProjectileMovement`))
  (`NiagaraComponent.SetAsset` (`self.Particle`) _projectileskilldata_bulletparticle true)
  (set `self.HitParticle` _projectileskilldata_hitparticle))