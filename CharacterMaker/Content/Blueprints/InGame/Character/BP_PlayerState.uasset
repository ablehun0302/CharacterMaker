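; Player state that holds a player's equipped items, skill slots, replicated nickname and death flag.
; Equipping or unequipping updates pawn meshes, pushes slot changes to the HUD through S2C events and recomputes summed stat bonuses for the player's stats.
; Skills are async-loaded Primary Data Assets that execute server logic, then trigger visuals via an S2M event.
; Death disables the pawn's movement.
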(event `OnDead`
  (params (InOwner :type "Actor Object Reference"))
  (set `self.bIsDead` true)
  (bind _asbp_player (cast `/Game/Blueprints/InGame/Character/BP_Player` InOwner))
  ; 움직임 제한
  (`/Game/Blueprints/InGame/Character/BP_Player.SetMovementFromState` _asbp_player "Dead")
  (`CharacterMovementComponent.DisableMovement` (`Character.CharacterMovement` _asbp_player)))

(event `S2C_OnEquippedItem`
  (params (InEquippedItem :type "/Game/Blueprints/InGame/Datas/Structure/ST_ItemInfo Structure"))
  (`/Game/Blueprints/InGame/Core/BP_HUD.OnAttatchItem` (`self.GetHUD`) InEquippedItem))

(event `S2C_OnUnequippedItem`
  (params (InItemSlot :type "/Game/Blueprints/InGame/Datas/Enum/E_ItemSlot Enum" :default "NewEnumerator0"))
  (`/Game/Blueprints/InGame/Core/BP_HUD.OnDetatchItem` (`self.GetHUD`) InItemSlot))

(event `S2M_UseSkill`
  (params (InSkillPDA :type "BaseSkillPDA Object Reference") (InPawn :type "Pawn Object Reference"))
  ; UseSkill
  (`BaseSkillPDA.SpawnVisualEffect` InSkillPDA InPawn))

(event `AttachSkill`
  (params (InSkillAssetID :type "PrimaryAssetId Structure") (InSkillSlot :type "/Game/Blueprints/InGame/Datas/Enum/E_SkillSlot Enum" :default "NewEnumerator0"))
  (bind _returnvalue (`KismetMathLibrary.Conv_ByteToInt` InSkillSlot))
  (bind _loaded (`AsyncActionLoadPrimaryAsset.AsyncLoadPrimaryAsset` InSkillAssetID)
    (:`Completed`
      (bind _asbase_skill_pda (cast `BaseSkillPDA` _loaded))
      ; 중복된 스킬이 아니면 스킬 장착
      (if (== (`KismetArrayLibrary.Array_Find` (`self.EquippedSkills`) _asbase_skill_pda) -1)
        (`KismetArrayLibrary.Array_Set` (`self.EquippedSkills`) _returnvalue _asbase_skill_pda)
        (`self.S2C_OnAttachSkill` _returnvalue (`BaseSkillPDA.SkillInfo` _asbase_skill_pda))))))

(event `S2C_OnAttachSkill`
  (params (InSlotIndex :type Integer) (InSkillInfo :type "SkillInfo Structure"))
  (`/Game/Blueprints/InGame/Core/BP_HUD.OnAttatchSkill` (`self.GetHUD`) InSlotIndex InSkillInfo))

(event `S2C_DetatchedSkill`
  (params (InSkillSlot :type "/Game/Blueprints/InGame/Datas/Enum/E_SkillSlot Enum" :default "NewEnumerator0"))
  ; DetatchSkill
  (`/Game/Blueprints/InGame/Core/BP_HUD.OnDetatchSkill` (`self.GetHUD`) InSkillSlot))

(fn `AttachCurrentAllItemMesh`
  (for _array_element (`self.EquippedItems`)
    (bind (_itemid _itemname _slot _itemtype _adjuststats _itemmesh _staticitemmesh) (break `/Game/Blueprints/InGame/Datas/Structure/ST_ItemInfo` _array_element))
    ; 아이템 외형 추가
    ;; 아이템이 스킨 형태면 몸에 붙이기
    (if (`|EnumEquality` _itemtype "NewEnumerator0")
      (`/Game/Blueprints/InGame/Character/BP_Player.AttachItemMesh` (`self.GetPlayer`) _slot _itemmesh)
      (else
        (`/Game/Blueprints/InGame/Character/BP_Player.AttachSwordMesh` (`self.GetPlayer`) _slot _staticitemmesh)))
    (`self.UpdateAdjustStats`)))

(fn `DetatchSkill`
  (params (InSkillSlot :type "/Game/Blueprints/InGame/Datas/Enum/E_SkillSlot Enum" :default "NewEnumerator0"))
  (bind _returnvalue (`KismetMathLibrary.Conv_ByteToInt` InSkillSlot))
  ; 해당 슬롯에 스킬이 있다면 장착 해제
  (`/Engine/EditorBlueprintResources/StandardMacros.IsValid` (`|GetArrayItem` (`self.EquippedSkills`) _returnvalue)
    (:`Is Valid`
      (`KismetArrayLibrary.Array_Set` (`self.EquippedSkills`) _returnvalue)
      (`self.S2C_DetatchedSkill` (`local.InSkillSlot`)))))

(fn `EquipItem`
  (params (InIndex :type Integer))
  ; 아이템 착용
  (bind _asbp_gamemode (cast `/Game/Blueprints/InGame/Core/BP_Gamemode` (`GameplayStatics.GetGameMode`)))
  (bind _output (`|GetArrayItem` (`/Game/Blueprints/InGame/Core/BP_Gamemode.ItemDatas` _asbp_gamemode) InIndex))
  (bind (_itemid _itemname _slot _itemtype _adjuststats _itemmesh _staticitemmesh) (break `/Game/Blueprints/InGame/Datas/Structure/ST_ItemInfo` _output))
  (`KismetArrayLibrary.Array_Set` (`self.EquippedItems`) (`KismetMathLibrary.Conv_ByteToInt` _slot) _output)
  ; 아이템 외형 추가
  ;; 아이템이 스킨 형태면 몸에 붙이기
  (if (`|EnumEquality` _itemtype "NewEnumerator0")
    (`/Game/Blueprints/InGame/Character/BP_Player.AttachItemMesh` (`self.GetPlayer`) _slot _itemmesh)
    (else
      (`/Game/Blueprints/InGame/Character/BP_Player.AttachSwordMesh` (`self.GetPlayer`) _slot _staticitemmesh)))
  ; 아이템 슬롯 UI 변경
  (`self.S2C_OnEquippedItem` _output)
  (`self.UpdateAdjustStats`))

(fn `GetHUD`
  (returns (OutHUD :type "/Game/Blueprints/InGame/Core/BP_HUD Object Reference"))
  (bind _returnvalue (`self.GetPlayerController`))
  (`/Engine/EditorBlueprintResources/StandardMacros.IsValid` (`self.Ref_HUD`)
    (:`Is Valid`
      (return (`self.Ref_HUD`)))
    (:`Is Not Valid`
      (`/Engine/EditorBlueprintResources/StandardMacros.IsValid` _returnvalue
        (:`Is Valid`
          (bind _asbp_hud (cast `/Game/Blueprints/InGame/Core/BP_HUD` (`PlayerController.GetHUD` _returnvalue)))
          (bind _output_get (set `self.Ref_HUD` _asbp_hud))
          (return _output_get))))))

(fn `GetPlayer`
  (returns (OutPlayer :type "/Game/Blueprints/InGame/Character/BP_Player Object Reference"))
  (bind _returnvalue (`self.GetPawn`))
  (`/Engine/EditorBlueprintResources/StandardMacros.IsValid` (`self.Ref_Player`)
    (:`Is Valid`
      (return (`self.Ref_Player`)))
    (:`Is Not Valid`
      (`/Engine/EditorBlueprintResources/StandardMacros.IsValid` _returnvalue
        (:`Is Valid`
          (bind _asbp_player (cast `/Game/Blueprints/InGame/Character/BP_Player` _returnvalue))
          (bind _output_get (set `self.Ref_Player` _asbp_player))
          (return _output_get))))))

(fn `OnRep_Nickname`
  (`self.OnUpdateNickname` (`self.Nickname`)))

(fn `UnequipItem`
  (params (InItemSlot :type "/Game/Blueprints/InGame/Datas/Enum/E_ItemSlot Enum" :default "NewEnumerator0"))
  ; 아이템 해제
  (`KismetArrayLibrary.Array_Set` (`self.EquippedItems`) (`KismetMathLibrary.Conv_ByteToInt` InItemSlot))
  ; 아이템 외형 해제
  (`/Game/Blueprints/InGame/Character/BP_Player.DetachItemMesh` (`self.GetPlayer`) (`local.InItemSlot`))
  (if (`|EnumEquality` (`local.InItemSlot`) "NewEnumerator6")
    (`/Game/Blueprints/InGame/Character/BP_Player.DetachSwordMesh` (`self.GetPlayer`)))
  ; 아이템 슬롯 UI 변경
  (`self.S2C_OnUnequippedItem` (`local.InItemSlot`))
  (`self.UpdateAdjustStats`))

(fn `UpdateAdjustStats`
  (locals (PreAdjustStats :type "CharacterStats Structure"))
  (set `local.PreAdjustStats` (`self.AdjustStats`))
  (set `self.AdjustStats` (struct))
  ; 장착한 아이템 변경시 현재 스탯 업뎃
  (for _array_element (`self.EquippedItems`)
    (set `self.AdjustStats` (`DataLibrary.AddCharacterStats` (`self.AdjustStats`) (`.AdjustStats_5_6C99EFC348664AD09190A09F84A50126` (break `/Game/Blueprints/InGame/Datas/Structure/ST_ItemInfo` _array_element)))))
  ; 현재 스탯 변경
  (bind _asbp_player (cast `/Game/Blueprints/InGame/Character/BP_Player` (`self.GetPawn`)))
  (`/Game/Blueprints/InGame/Components/BP_CharacterStats.UpdateMaxStats` (`/Game/Blueprints/InGame/Character/BP_Player.BP_PlayerStats` _asbp_player) (`local.PreAdjustStats`) (`self.AdjustStats`)))

(fn `UserConstructionScript`
  (`|ExecutionSequence`
    (:`then_1`
      ; 캐릭터 아이템 슬롯 초기화
      (foreach `/Game/Blueprints/InGame/Datas/Enum/E_ItemSlot` false
        (:`LoopBody`
          (`KismetArrayLibrary.Array_Add` (`self.EquippedItems`) (make `/Game/Blueprints/InGame/Datas/Structure/ST_ItemInfo` "None" "None" "NewEnumerator0" "NewEnumerator0" (struct) null null null)))))
    (:`then_2`
      ; 스킬 슬롯 초기화
      (`KismetArrayLibrary.Array_Resize` (`self.EquippedSkills`) (enumcount `/Game/Blueprints/InGame/Datas/Enum/E_SkillSlot`)))))

(fn `UseSkill`
  (params (InSkillSlot :type "/Game/Blueprints/InGame/Datas/Enum/E_SkillSlot Enum" :default "NewEnumerator0"))
  (bind _returnvalue (`self.GetPawn`))
  (bind _output (`|GetArrayItem` (`self.EquippedSkills`) (`KismetMathLibrary.Conv_ByteToInt` InSkillSlot)))
  (`/Engine/EditorBlueprintResources/StandardMacros.IsValid` _output
    (:`Is Valid`
      (bind _returnvalue_2 (`BaseSkillPDA.ExecuteSkillServer` _output _returnvalue))
      (if _returnvalue_2
        (`self.S2M_UseSkill` _output _returnvalue)))))