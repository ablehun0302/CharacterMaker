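; BP_Gamemode is the game mode that supplies item and skill data, respawns players and spawns monsters.
; It caches DT_Items rows on BeginPlay and skill asset IDs at construction, attaching skills to player states by slot index.
; RestartClient destroys the old pawn and sword, clears the death flag and possesses a new BP_Player.
; BeginPlay also starts a looping timer, and SpawnMonster adds slimes at random reachable points while MonsterPool is below its cap.
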(event `self.ReceiveBeginPlay`
  (`|ExecutionSequence`
    (:`then_0`
      ; 아이템 데이터
      (bind _outrownames (`DataTableFunctionLibrary.GetDataTableRowNames` "/Game/Blueprints/InGame/Datas/DataTable/DT_Items.DT_Items"))
      (for _array_element _outrownames
        (bind _returnvalue (`|GetDataTableRow` "/Game/Blueprints/InGame/Datas/DataTable/DT_Items.DT_Items" _array_element)
          (:`then`
            (`KismetArrayLibrary.Array_Add` (`self.ItemDatas`) (make `/Game/Blueprints/InGame/Datas/Structure/ST_ItemInfo` _array_element (break `/Game/Blueprints/InGame/Datas/Structure/ST_ItemData` _returnvalue) (`.Slot_13_F1E0FF0D4685ADB0C5EC70993474033B` (break `/Game/Blueprints/InGame/Datas/Structure/ST_ItemData` _returnvalue)) (`.ItemType_27_AFDC59834B816EA848B5B4880878D4D4` (break `/Game/Blueprints/InGame/Datas/Structure/ST_ItemData` _returnvalue)) (`.AdjustStats_9_288C978C4D8C40B55295F3B129592EB2` (break `/Game/Blueprints/InGame/Datas/Structure/ST_ItemData` _returnvalue)) (`.ItemMesh_20_56B5E5774D5F5B35A63BB1AF3D3F15E1` (break `/Game/Blueprints/InGame/Datas/Structure/ST_ItemData` _returnvalue)) (`.StaticItemMesh_31_44C1E1E94C1434B69E0D70A2E1D04F51` (break `/Game/Blueprints/InGame/Datas/Structure/ST_ItemData` _returnvalue)) (`.ItemImage_24_C9ADD5254F05D3E7C89801A47058A2AD` (break `/Game/Blueprints/InGame/Datas/Structure/ST_ItemData` _returnvalue))))))))
    (:`then_1`
      (`KismetSystemLibrary.K2_SetTimerDelegate` (`|CreateDelegate` :!event `SpawnMonster`) 5.0 true))))

(event `GetSkillData`
  (params (InCaster :type "/Game/Blueprints/InGame/Character/BP_Controller Object Reference") (InSlotIndex :type Integer) (InSkillSlot :type "/Game/Blueprints/InGame/Datas/Enum/E_SkillSlot Enum" :default "NewEnumerator0"))
  ; 스킬 가져오기
  (`/Game/Blueprints/InGame/Character/BP_PlayerState.AttachSkill` (`/Game/Blueprints/InGame/Character/BP_Controller.GetBP_PlayerState` InCaster) (`|GetArrayItem` (`self.SkillAssetDatas`) InSlotIndex) InSkillSlot))

(fn `OnPlayerDead`
  (params (InPlayerState :type "/Game/Blueprints/InGame/Character/BP_PlayerState Object Reference"))
  (locals (Ref_Pawn :type "Pawn Object Reference"))
  (set `local.Ref_Pawn` (`PlayerState.GetPawn` InPlayerState)))

(fn `RestartClient`
  (params (InPlayerController :type "PlayerController Object Reference"))
  (locals (Ref_DeadPawn :type "Pawn Object Reference"))
  ; 죽은 캐릭터 삭제
  (bind _asbp_player (cast `/Game/Blueprints/InGame/Character/BP_Player` (`Controller.K2_GetPawn` InPlayerController)))
  (`self.K2_DestroyActor` (`/Game/Blueprints/InGame/Character/BP_Player.Ref_Sword` _asbp_player))
  (`self.K2_DestroyActor` _asbp_player)
  ; 죽은 상태 초기화
  (bind _asbp_player_state (cast `/Game/Blueprints/InGame/Character/BP_PlayerState` (`Controller.PlayerState` (`local.InPlayerController`))))
  (set `/Game/Blueprints/InGame/Character/BP_PlayerState.bIsDead` false _asbp_player_state)
  ; 캐릭터 생성
  (bind _returnvalue (`|SpawnActorFromClass` "/Game/Blueprints/InGame/Character/BP_Player.BP_Player_C" (`self.GetTransform` (`self.K2_FindPlayerStart` (`local.InPlayerController`))) "Undefined" "MultiplyWithRoot" (`local.InPlayerController`) null))
  (`Controller.Possess` (`local.InPlayerController`) _returnvalue))

(fn `SpawnMonster`
  ; 필드에 몬스터가 충분하지 않다면 몬스터 생성
  (if (< (`KismetArrayLibrary.Array_Length` (`self.MonsterPool`)) 10)
    (bind _returnvalue (`|SpawnActorFromClass` "/Game/Blueprints/InGame/Monster/BP_Slime.BP_Slime_C" (`KismetMathLibrary.MakeTransform` (`NavigationSystemV1.K2_GetRandomReachablePointInRadius` (`KismetMathLibrary.MakeVector` -7590.0 4380.0 550.0) 3000.0 null null) (`KismetMathLibrary.MakeRotator` 0.0 0.0 (`KismetMathLibrary.RandomFloatInRange` 0.0 360.0))) "AdjustIfPossibleButAlwaysSpawn" "MultiplyWithRoot" self null))
    (`/Engine/EditorBlueprintResources/StandardMacros.IsValid` _returnvalue
      (:`Is Valid`
        (`KismetArrayLibrary.Array_Add` (`self.MonsterPool`) _returnvalue)))))

(fn `UserConstructionScript`
  ; 스킬 데이터
  (bind _outprimaryassetidlist (`KismetSystemLibrary.GetPrimaryAssetIdList` "Skill"))
  (set `self.SkillAssetDatas` _outprimaryassetidlist))